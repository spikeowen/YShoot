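; Level manager actor that streams the game's levels in sequence, starting at Level1A and returning to it after Level5.
; Tick polls the first-person character's LevelChange flag, increments its CurrentLevel, then after a delay switches on that number without ever resetting it.
; LoadLevel unloads and hides the previous streaming level before loading and showing the next.
; RespawnPlayer also runs delayed, teleporting the character to a hard-coded spot and resetting its timer if Respawn is set.
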(event `self.ReceiveBeginPlay`
  (`self.LoadLevel` "Level1A")
  (bind _returnvalue (`GameplayStatics.GetActorOfClass` "/Game/FirstPerson/Blueprints/BP_FirstPersonCharacter.BP_FirstPersonCharacter_C"))
  (set `self.Player` _returnvalue))

(event `self.ReceiveTick`
  (params (DeltaSeconds :type "Float (single-precision)"))
  (bind _player (`self.Player`))
  (if (`/Game/FirstPerson/Blueprints/BP_FirstPersonCharacter.LevelChange` (`self.Player`))
    (bind _output_get (set `/Game/FirstPerson/Blueprints/BP_FirstPersonCharacter.CurrentLevel` (+ (`/Game/FirstPerson/Blueprints/BP_FirstPersonCharacter.CurrentLevel` _player) 1) _player))
    (`|ExecutionSequence`
      (:`then_0`
        (set `/Game/FirstPerson/Blueprints/BP_FirstPersonCharacter.LevelChange` false (`self.Player`))
        (`KismetSystemLibrary.Delay` 2.0)
        (`self.RespawnPlayer`))
      (:`then_1`
        (`KismetSystemLibrary.Delay` 2.0)
        (switch `int` _output_get
          (:`1`
            (`self.LoadLevel` "Level2")
            (`KismetSystemLibrary.PrintString` "Level Changed"))
          (:`2`
            (`self.LoadLevel` "Level3")
            (`KismetSystemLibrary.PrintString` "Level Changed"))
          (:`3`
            (`self.LoadLevel` "Level4")
            (`KismetSystemLibrary.PrintString` "Level Changed"))
          (:`4`
            (`self.LoadLevel` "Level5")
            (`KismetSystemLibrary.PrintString` "Level Changed"))
          (:`5`
            (`self.LoadLevel` "Level1A")
            (`KismetSystemLibrary.PrintString` "Level Changed")))))))

(fn `LoadLevel`
  (params (Level :type String))
  (bind _returnvalue (`GameplayStatics.GetStreamingLevel` (`KismetStringLibrary.Conv_StringToName` (`self.LevelLoaded`))))
  (`|ExecutionSequence`
    (:`then_0`
      (set `LevelStreaming.bShouldBeLoaded` false _returnvalue)
      (set `LevelStreaming.bShouldBeVisible` false _returnvalue))
    (:`then_1`
      (bind _output_get (set `self.LevelLoaded` Level))
      (bind _returnvalue_2 (`GameplayStatics.GetStreamingLevel` (`KismetStringLibrary.Conv_StringToName` _output_get)))
      (set `LevelStreaming.bShouldBeLoaded` true _returnvalue_2)
      (set `LevelStreaming.bShouldBeVisible` true _returnvalue_2))))

(fn `RespawnPlayer`
  (bind _as_bp_first_person_character (`self.As BP First Person Character`))
  (bind _asbp_first_person_character (cast `/Game/FirstPerson/Blueprints/BP_FirstPersonCharacter` (`GameplayStatics.GetPlayerCharacter` 0)))
  (bind _output_get (set `self.As BP First Person Character` _asbp_first_person_character))
  (if (`/Game/FirstPerson/Blueprints/BP_FirstPersonCharacter.Respawn` _output_get)
    (`self.K2_SetActorLocationAndRotation` _as_bp_first_person_character (2700.0 250.0 192.0) (struct :`Yaw` 230.0) false true)
    (`/Game/YShootContent/THIS_IS_THE_HUD.ResetTimer` (`/Game/FirstPerson/Blueprints/BP_FirstPersonCharacter.NewVar` _as_bp_first_person_character))
    (set `/Game/FirstPerson/Blueprints/BP_FirstPersonCharacter.Respawn` false _as_bp_first_person_character)))

(fn `UserConstructionScript`)