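; BP_Enemy is an enemy actor whose destruction stops the player's timer and flags a level change.
; On BeginPlay it caches the first-person character and binds Die to its own OnDestroyed event.
; Die stops the timer through a reference held by the character, plays a sped-up FadeToBlack level sequence, then sets the character's Respawn and LevelChange flags.
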(event `self.ReceiveBeginPlay`
  (bind _returnvalue (`GameplayStatics.GetActorOfClass` "/Game/FirstPerson/Blueprints/BP_FirstPersonCharacter.BP_FirstPersonCharacter_C"))
  (set `self.NewVar` _returnvalue)
  (add `self.OnDestroyed` (delegate `Die`)))

(event `Die` :!signature `self.OnDestroyed`
  (params (DestroyedActor :type "Actor Object Reference"))
  (bind _newvar (`self.NewVar`))
  (`/Game/YShootContent/THIS_IS_THE_HUD.StopTimer` (`/Game/FirstPerson/Blueprints/BP_FirstPersonCharacter.NewVar` (`self.NewVar`)))
  (`|ExecutionSequence`
    (:`then_0`
      (bind (_outactor _returnvalue) (`LevelSequencePlayer.CreateLevelSequencePlayer` "/Game/YShootContent/Animation/FadeToBlack.FadeToBlack" (make `MovieSceneSequencePlaybackSettings` false (struct) 2.0)))
      (`MovieSceneSequencePlayer.Play` _returnvalue))
    (:`then_1`
      (set `/Game/FirstPerson/Blueprints/BP_FirstPersonCharacter.Respawn` true _newvar)
      (set `/Game/FirstPerson/Blueprints/BP_FirstPersonCharacter.LevelChange` true _newvar))))

(fn `UserConstructionScript`)